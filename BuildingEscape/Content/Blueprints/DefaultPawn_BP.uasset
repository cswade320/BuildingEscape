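; DefaultPawn_BP is the player pawn that manages the in-game HUD and the win screen.
; On BeginPlay it creates MyHUD_BP and adds it to the viewport, and pre-creates WinScreenMenu_BP without showing it.
; Its WinGame event swaps the HUD for the win screen, switches input to UI-only, shows the mouse cursor and pauses the game.
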(event Custom|WinGame
  (bind _returnvalue (Game|GetPlayerController 0))
  (bind _winscreenreference (Variables|Default|GetWinScreenReference))
  (Widget|RemovefromParent (Variables|Default|GetMyHudReference))
  (UserInterface|Viewport|AddtoViewport _winscreenreference 0)
  (Input|SetInputModeUIOnly _returnvalue _winscreenreference "DoNotLock")
  (Variables|/Script/Engine.PlayerController|SetbShowMouseCursor _returnvalue true)
  (Game|SetGamePaused true))

(event EventBeginPlay
  (bind _returnvalue (Game|GetPlayerController 0))
  (bind _returnvalue_2 (UserInterface|CreateWidget "/Game/Blueprints/MyHUD_BP.MyHUD_BP_C" _returnvalue))
  (bind _output_get (Variables|Default|SetMyHudReference _returnvalue_2))
  (UserInterface|Viewport|AddtoViewport _output_get 0)
  (bind _returnvalue_3 (UserInterface|CreateWidget "/Game/Blueprints/WinScreenMenu_BP.WinScreenMenu_BP_C" _returnvalue))
  (Variables|Default|SetWinScreenReference _returnvalue_3))

(event Collision|EventActorBeginOverlap
  (params (OtherActor :type Actor%20Object%20Reference)))

(event EventTick
  (params (DeltaSeconds :type Float%20%28single-precision%29)))

(fn ConstructionScript)